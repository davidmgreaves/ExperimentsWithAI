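; BP_EnemyTurret is an enemy turret actor that turns to face and fires at a first-person character it sees.
; Each PawnSensing sighting snaps the actor toward the character, then spawns a FirstPersonProjectile at ProjectileSpawnLocation if SpawnProjectile is true.
; The impulse and the reload cooldown that toggles SpawnProjectile are disconnected, so neither runs.
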(event `self.PawnSensing.OnSeePawn`
  (params (Pawn :type "Pawn Object Reference"))
  (bind _asfirst_person_character (cast `/Game/FirstPersonBP/Blueprints/FirstPersonCharacter` Pawn))
  (`|ExecutionSequence`
    (:`then_0`
      (`self.K2_SetActorRotation` (`KismetMathLibrary.FindLookAtRotation` (`self.K2_GetActorLocation`) (`self.K2_GetActorLocation` _asfirst_person_character))))
    (:`then_1`
      (if (`self.SpawnProjectile`)
        (bind _returnvalue (`|SpawnActorFromClass` "/Game/FirstPersonBP/Blueprints/FirstPersonProjectile.FirstPersonProjectile_C" (`SceneComponent.K2_GetComponentToWorld` (`self.ProjectileSpawnLocation`)) "Undefined" "OverrideRootScale"))))))

(fn `UserConstructionScript`)