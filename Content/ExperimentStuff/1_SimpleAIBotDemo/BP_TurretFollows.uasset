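; Demo AI turret that turns to face a FirstPersonCharacter it sees and spawns a projectile at its muzzle point.
; Pawn sensing drives the rotation, with spawning gated by the SpawnProjectile flag.
; BeginPlay stores three marker positions and picks one at random.
; The timeline patrol that lerps between them and the projectile impulse with reload cooldown are both unconnected, so neither runs.
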(event `self.PawnSensing.OnSeePawn`
  (params (Pawn :type "Pawn Object Reference"))
  ;[1 1 1] Look At and Shoot
  (bind _asfirst_person_character (cast `/Game/FirstPersonBP/Blueprints/FirstPersonCharacter` Pawn))
  (`|ExecutionSequence`
    (:`then_0`
      (`self.K2_SetActorRotation` (`KismetMathLibrary.FindLookAtRotation` (`self.K2_GetActorLocation`) (`self.K2_GetActorLocation` _asfirst_person_character))))
    (:`then_1`
      (if (`self.SpawnProjectile`)
        (bind _returnvalue (`|SpawnActorFromClass` "/Game/FirstPersonBP/Blueprints/FirstPersonProjectile.FirstPersonProjectile_C" (`SceneComponent.K2_GetComponentToWorld` (`self.ProjectileSpawnLocation`)) "Undefined" "OverrideRootScale"))))))

(event `self.ReceiveBeginPlay`
  ;[1 1 1] Set Enemy Locations
  (set `self.EnemyLocations` (`|MakeArray` (`SceneComponent.K2_GetComponentLocation` (`self.Position1`)) (`SceneComponent.K2_GetComponentLocation` (`self.Position2`)) (`SceneComponent.K2_GetComponentLocation` (`self.Position3`))))
  (`self.GetRandomLocation`))

(fn `GetRandomLocation`
  (set `self.CurrentEnemyLocation` (`KismetMathLibrary.RandomInteger` (`KismetArrayLibrary.Array_Length` (`self.EnemyLocations`)))))

(fn `UserConstructionScript`)